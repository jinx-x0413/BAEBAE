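; Game instance that holds session settings and work metrics, saving them through a BP_SG save object created at Init.
; InitInstanceVar stores map and difficulty and has presets for aerosol, vibration and noise flags, though its switch reads a constant 1 rather than Difficulty.
; EndGame calls DisplayResult, then writes timing, accuracy, block, wind and condition data to the save slot.
; Result display functions are empty, and loading only checks the save reference.
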(event `self.ReceiveInit`
  (`self.Init`))

(fn `DisplayResult`)

(fn `DisplayResultTable`)

(fn `EndGame`
  (`self.DisplayResult`)
  (`self.SaveDataToSG`))

(fn `Init`
  (bind _returnvalue (`GameplayStatics.CreateSaveGameObject` "/Game/BAEBAE/GameMode/BP_SG.BP_SG_C"))
  (bind _output_get (set `self.SGRef` _returnvalue))
  (`KismetSystemLibrary.PrintString` (`KismetStringLibrary.Conv_IntToString` (`/Game/BAEBAE/GameMode/BP_SG.UserIndex` _output_get))))

(fn `InitInstanceVar`
  (params (CurrentMap :type "/Game/BAEBAE/Enum/E_Maps Enum" :default "NewEnumerator0") (Difficulty :type "/Game/BAEBAE/Enum/E_Difficulties Enum" :default "NewEnumerator0"))
  (`|ExecutionSequence`
    (:`then_0`
      (set `self.E_Map` CurrentMap))
    (:`then_1`
      (set `self.E_Difficulty` Difficulty)
      (switch `/Game/BAEBAE/Enum/E_Difficulties` "NewEnumerator0"
        (:`NewEnumerator0`
          (set `self.bIsAerosol` true)
          (set `self.bIsVibration` false)
          (set `self.bIsNoise` false))
        (:`NewEnumerator1`
          (set `self.bIsAerosol` true)
          (set `self.bIsVibration` true)
          (set `self.bIsNoise` false))
        (:`NewEnumerator2`
          (set `self.bIsAerosol` true)
          (set `self.bIsVibration` false)
          (set `self.bIsNoise` true))
        (:`NewEnumerator3`
          (set `self.bIsAerosol` true)
          (set `self.bIsVibration` true)
          (set `self.bIsNoise` false))
        (:`NewEnumerator4`
          (set `self.bIsAerosol` true)
          (set `self.bIsVibration` true)
          (set `self.bIsNoise` true))))))

(fn `LoadDataFromSG`
  (`/Engine/EditorBlueprintResources/StandardMacros.IsValid` (`self.SGRef`)
    (:`Is Not Valid`
      (`KismetSystemLibrary.PrintString` "SGRef Invalid"))))

(fn `SaveDataToSG`
  (bind _sgref (`self.SGRef`))
  (`/Engine/EditorBlueprintResources/StandardMacros.IsValid` (`self.SGRef`)
    (:`Is Valid`
      (`/Game/BAEBAE/GameMode/BP_SG.UpdateData` (`self.SGRef`) (`self.TotalWorkTime`) (`self.EachWorkTime`) (`self.WorkInterval`) (`self.WorkAccuracy`) (`self.TotalBlocks`) (`self.WindDirection`) (`self.E_Difficulty`) (`self.E_Map`) (`self.bIsAerosol`) (`self.bIsNoise`) (`self.bIsVibration`))
      (`GameplayStatics.SaveGameToSlot` _sgref (`/Game/BAEBAE/GameMode/BP_SG.SlotName` _sgref) (`/Game/BAEBAE/GameMode/BP_SG.UserIndex` _sgref)))
    (:`Is Not Valid`
      (`KismetSystemLibrary.PrintString` "SGRef Invalid"))))