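; BP_SG is a data holder for work-session settings, covering timing, accuracy, block count, wind direction, difficulty and map.
; It also stores toggles for aerosol, noise and vibration.
; Its single UpdateData function copies all incoming values into the matching variables in one call, with no validation or further logic.
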(fn `UpdateData`
  (params (TotalWorkTime :type "Float (double-precision)") (EachWorkTime :type "Float (double-precision)") (WorkInterval :type "Float (double-precision)") (WorkAccuracy :type "Float (double-precision)") (TotalBlocks :type Integer) (WindDirection :type "Float (double-precision)") (Difficulty :type "/Game/BAEBAE/Enum/E_Difficulties Enum" :default "NewEnumerator0") (Map :type "/Game/BAEBAE/Enum/E_Maps Enum" :default "NewEnumerator0") (bIsAerosol :type Boolean) (bIsNoise :type Boolean) (bIsVibration :type Boolean))
  (set `self.TotalWorkTime` TotalWorkTime)
  (set `self.EachWorkTime` EachWorkTime)
  (set `self.WorkInterval` WorkInterval)
  (set `self.WorkAccuracy` WorkAccuracy)
  (set `self.TotalBlocks` TotalBlocks)
  (set `self.WindDirection` WindDirection)
  (set `self.Difficulty` Difficulty)
  (set `self.Map` Map)
  (set `self.bIsAerosol` bIsAerosol)
  (set `self.bIsNoise` bIsNoise)
  (set `self.bIsVibration` bIsVibration))