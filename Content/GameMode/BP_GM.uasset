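; Game mode Blueprint that sets up the in-game HUD and shows the selected map and difficulty.
; On BeginPlay it caches the BP_GI game instance, then creates UMG_Game only when the current level is "Game".
; It then writes the game instance's map and difficulty enums into the widget's text blocks, without checking that the widget was created.
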(event `self.ReceiveBeginPlay`
  (`self.Init`))

(fn `Init`
  (bind _asbp_gi (cast `/Game/BAEBAE/GameMode/BP_GI` (`GameplayStatics.GetGameInstance`)))
  (set `self.GIRef` _asbp_gi)
  (`self.InitUI`)
  (`self.InitGameStateText`))

(fn `InitGameStateText`
  (`TextBlock.SetText` (`/Game/BAEBAE/UMG/UMG_Game.TB_State_Map` (`self.UIGameRef`)) (`KismetTextLibrary.Conv_StringToText` (`|GetEnumeratorNameAsString` (`/Game/BAEBAE/GameMode/BP_GI.E_Map` (`self.GIRef`)))))
  (`TextBlock.SetText` (`/Game/BAEBAE/UMG/UMG_Game.TB_State_Difficulty` (`self.UIGameRef`)) (`KismetTextLibrary.Conv_StringToText` (`KismetStringLibrary.Concat_StrStr` "난이도 : " (`|GetEnumeratorNameAsString` (`/Game/BAEBAE/GameMode/BP_GI.E_Difficulty` (`self.GIRef`)))))))

(fn `InitUI`
  (bind _returnvalue (`GameplayStatics.GetCurrentLevelName` true))
  (if (`KismetStringLibrary.EqualEqual_StrStr` _returnvalue "Game")
    (bind _returnvalue_2 (`|CreateWidget` "/Game/BAEBAE/UMG/UMG_Game.UMG_Game_C"))
    (bind _output_get (set `self.UIGameRef` _returnvalue_2))
    (`UserWidget.AddToViewport` _output_get 0)))

(fn `NewFunction`)

(fn `UserConstructionScript`)