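; BP_FloorCube is a destructible floor cube that the drill breaks through.
; When the Floor component begins overlapping a BP_Drill that is drilling, it increments and prints a hit counter.
; Once the count reaches MaxHP, it notifies the drill through DestroySuccess and destroys itself.
; An author note proposes adding a small collision volume so only hits on that spot count.
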(event `self.Floor.OnComponentBeginOverlap`
  (params (OverlappedComponent :type "PrimitiveComponent Object Reference") (OtherActor :type "Actor Object Reference") (OtherComp :type "PrimitiveComponent Object Reference") (OtherBodyIndex :type Integer) (bFromSweep :type Boolean) (SweepResult :type "HitResult Structure (by ref)"))
  (bind _asbp_drill (cast `/Game/Blueprints/EquipMent/BP_Drill` OtherActor))
  (if (`/Game/Blueprints/EquipMent/BP_Drill.Drilling` _asbp_drill)
    (bind _result (`/Engine/EditorBlueprintResources/StandardMacros.IncrementInt` (`self.CountToDestroy`))
      (:`  `
        (`KismetSystemLibrary.PrintString` (`KismetStringLibrary.Conv_IntToString` _result))
        (if (>= (`self.CountToDestroy`) (`self.MaxHP`))
          (`/Game/Blueprints/EquipMent/BP_Drill.DestroySuccess` _asbp_drill)
          (`self.K2_DestroyActor`))))))

(fn `UserConstructionScript`)