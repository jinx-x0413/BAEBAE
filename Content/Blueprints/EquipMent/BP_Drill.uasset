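; BP_Drill is a drill equipment actor that attaches to the first-person player on capsule overlap.
; Vibrating runs a Gate and Delay loop that alternately offsets the drill, player mesh and camera to simulate shaking.
; Completed closes the gate and undoes any pending offset so everything returns to rest.
; DestroySuccess, for a successfully destroyed structure, updates the count on that player's BP_FirstPlayerState.
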(event `DestroySuccess`
  (bind _firstplayerref (`self.FirstPlayerRef`))
  ;[1 1 1] 구조물을 부시는데 성공했을때
  (`/Engine/EditorBlueprintResources/StandardMacros.IsValid` _firstplayerref
    (:`Is Valid`
      (bind _asbp_first_player_state (cast `/Game/Blueprints/FirstPerson/BP_FirstPlayerState` (`Pawn.PlayerState` _firstplayerref)))
      (`/Game/Blueprints/FirstPerson/BP_FirstPlayerState.UpdateCount` _asbp_first_player_state))))

(event `self.Capsule.OnComponentBeginOverlap`
  (params (OverlappedComponent :type "PrimitiveComponent Object Reference") (OtherActor :type "Actor Object Reference") (OtherComp :type "PrimitiveComponent Object Reference") (OtherBodyIndex :type Integer) (bFromSweep :type Boolean) (SweepResult :type "HitResult Structure (by ref)"))
  ;[1 1 1] Player가 CapsuleComponent에 오버랩시
  (bind _asbp_first_player (cast `/Game/Blueprints/FirstPerson/BP_FirstPlayer` OtherActor))
  (bind _output_get (set `self.FirstPlayerRef` _asbp_first_player))
  (`/Game/Blueprints/FirstPerson/BP_FirstPlayer.AttachEquip` _output_get self (`self.EquipType`)))

(event `Vibrating`
  (bind _firstplayerref (`self.FirstPlayerRef`))
  (bind _firstpersonmesh (`/Game/Blueprints/FirstPerson/BP_FirstPlayer.FirstPersonMesh` _firstplayerref))
  (bind _firstpersoncamera (`/Game/Blueprints/FirstPerson/BP_FirstPlayer.FirstPersonCamera` _firstplayerref))
  ;[1 1 1] 드릴 진동
  (set `self.Drilling` true)
  (`|ExecutionSequence`
    (:`then_0`
      (goto _label :!via `Open`))
    (:`then_1`
      (`/Engine/EditorBlueprintResources/StandardMacros.Gate` true :!label _label
        (:`Exit`
          (`|ExecutionSequence`
            (:`then_0`
              (`KismetSystemLibrary.Delay` 0.05)
              (goto _label))
            (:`then_1`
              (if (`self.DoDown`)
                ;;[1 1 1] 난이도 별로 움직이는 정도 바꾸면 될듯
                (`self.K2_AddActorLocalOffset` (0.0 0.0 -5.0))
                (`SceneComponent.K2_AddLocalOffset` _firstpersonmesh (0.0 0.0 -5.0) false false)
                (`SceneComponent.K2_AddLocalOffset` _firstpersoncamera (1.0 0.0 0.0) false false)
                (set `self.DoDown` false)
                (else
                  (`self.K2_AddActorLocalOffset` (0.0 0.0 5.0) :!label _label_2)
                  (`SceneComponent.K2_AddLocalOffset` _firstpersonmesh (0.0 0.0 5.0) false false)
                  (`SceneComponent.K2_AddLocalOffset` _firstpersoncamera (-1.0 0.0 0.0) false false)
                  (set `self.DoDown` true))))))))))

(event `Completed`
  ;[1 1 1] 드릴 진동
  (set `self.Drilling` false)
  (`|ExecutionSequence`
    (:`then_0`
      (goto _label :!via `Close`))
    (:`then_1`
      (if (not (`self.DoDown`))
        (goto _label_2)))))

(fn `UserConstructionScript`)