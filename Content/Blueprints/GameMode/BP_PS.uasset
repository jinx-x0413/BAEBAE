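; BP_PS, apparently a player state, tracks a player's block-destruction count and average work time per block.
; UpdateEachWorkTime increments BlockDestroyed, then folds the passed-in work time into EachWorkTime as an incremental running mean, without storing individual samples.
; The construction script is empty.
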(fn `UpdateEachWorkTime`
  (params (CurrentWorkTime :type "Float (double-precision)"))
  ;[0 0 0] UpdateDestroyedBlocks
  (set `self.BlockDestroyed` (+ (`self.BlockDestroyed`) 1))
  ;[0 0 0] Avg. EachWorkTime
  (set `self.EachWorkTime` (/ (+ CurrentWorkTime (* (`self.EachWorkTime`) (- (`self.BlockDestroyed`) 1))) (`self.BlockDestroyed`))))

(fn `UserConstructionScript`)