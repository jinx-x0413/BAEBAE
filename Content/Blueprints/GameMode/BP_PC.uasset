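; BP_PC is a player controller Blueprint that handles pausing the game from the P key.
; Pressing P calls ToggleGamePause, which flips the paused state, switches between game-only and UI-only input, and toggles the mouse cursor.
; The same press removes the WBP_InGamePause widget if its stored reference is valid, otherwise creates it and adds it to the viewport.
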(event `Key|P`
  (params (Key :type "Key Structure"))
  (:`Pressed`
    (`self.ToggleGamePause`)
    (`/Engine/EditorBlueprintResources/StandardMacros.IsValid` (`self.UIPauseRef`)
      (:`Is Valid`
        (`Widget.RemoveFromParent` (`self.UIPauseRef`)))
      (:`Is Not Valid`
        (bind _returnvalue (`|CreateWidget` "/Game/Blueprints/UMG/WBP_InGamePause.WBP_InGamePause_C"))
        (bind _output_get (set `self.UIPauseRef` _returnvalue))
        (`UserWidget.AddToViewport` _output_get 0)))))

(fn `ToggleGamePause`
  (if (`GameplayStatics.IsGamePaused`)
    (`GameplayStatics.SetGamePaused` false)
    (`WidgetBlueprintLibrary.SetInputMode_GameOnly` (`GameplayStatics.GetPlayerController` 0))
    (set `self.bShowMouseCursor` false)
    (else
      (`GameplayStatics.SetGamePaused` true)
      (`WidgetBlueprintLibrary.SetInputMode_UIOnlyEx` (`GameplayStatics.GetPlayerController` 0) null)
      (set `self.bShowMouseCursor` true))))

(fn `UserConstructionScript`)