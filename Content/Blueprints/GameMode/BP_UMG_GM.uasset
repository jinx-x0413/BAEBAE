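; BP_UMG_GM is a game mode Blueprint that brings up the menu UI when play begins.
; On BeginPlay it stores the current level name, and if it is "Menu" it creates the UMG_Menu widget and adds it to the viewport.
; It also switches the player controller to UI-only input and shows the mouse cursor, whatever the level name.
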(event `self.ReceiveBeginPlay`
  (bind _returnvalue (`GameplayStatics.GetPlayerController` 0))
  (`|ExecutionSequence`
    (:`then_0`
      (bind _returnvalue_2 (`GameplayStatics.GetCurrentLevelName` true))
      (set `self.CurrentLevelName` _returnvalue_2)
      (`|ExecutionSequence`
        (:`then_0`
          (if (`KismetStringLibrary.EqualEqual_StrStr` (`self.CurrentLevelName`) "Menu")
            (bind _returnvalue_3 (`|CreateWidget` "/Game/Blueprints/UMG/UMG_Menu.UMG_Menu_C"))
            (bind _output_get (set `self.UMGRef` _returnvalue_3))
            (`UserWidget.AddToViewport` _output_get 0)))))
    (:`then_1`
      (`WidgetBlueprintLibrary.SetInputMode_UIOnlyEx` _returnvalue null)
      (set `PlayerController.bShowMouseCursor` true _returnvalue))))

(fn `UserConstructionScript`)