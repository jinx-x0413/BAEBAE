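; BP_GM is a game mode Blueprint that sets up the session and its manual UI when play begins.
; It copies the map and difficulty selections from BP_GI, the game instance, then passes them into BP_GS, the game state, through InitGameState and gives it a back-reference to itself.
; It then creates the UMG_Manual widget, links it back to the game mode and adds it to the viewport.
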(event `self.ReceiveBeginPlay`
  (`self.InitGameInstances`)
  (`self.CreateManualWidget`))

(fn `CreateManualWidget`
  (bind _returnvalue (`|CreateWidget` "/Game/Blueprints/UMG/UMG_Manual.UMG_Manual_C"))
  (bind _output_get (set `self.UMGManualRef` _returnvalue))
  (set `/Game/Blueprints/UMG/UMG_Manual.GMRef` self _output_get)
  (`UserWidget.AddToViewport` _output_get 0))

(fn `InitGameInstances`
  (`|ExecutionSequence`
    (:`then_0`
      (bind _asbp_gi (cast `/Game/Blueprints/GameMode/BP_GI` (`GameplayStatics.GetGameInstance`)))
      (set `self.GIRef` _asbp_gi)
      (set `self.E_Maps` (`/Game/Blueprints/GameMode/BP_GI.E_Maps` (`self.GIRef`)))
      (set `self.E_DIfficulties` (`/Game/Blueprints/GameMode/BP_GI.E_Difficulties` (`self.GIRef`))))
    (:`then_1`
      (bind _asbp_gs (cast `/Game/Blueprints/GameMode/BP_GS` (`GameplayStatics.GetGameState`)))
      (bind _output_get (set `self.GSRef` _asbp_gs))
      (set `/Game/Blueprints/GameMode/BP_GS.GMRef` self _output_get)
      (`/Game/Blueprints/GameMode/BP_GS.InitGameState` _output_get (`self.E_Maps`) (`self.E_DIfficulties`)))))

(fn `UserConstructionScript`)