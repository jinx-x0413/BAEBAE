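; BP_GS is a game state Blueprint that holds the environment and difficulty settings for the selected map.
; InitGameState sets the open-area flag from the map (Inside or Outside) and maps five difficulty levels to vibration, noise and dynamic wind flags.
; It then calls UpdateWind, which picks a random unit wind direction only when dynamic wind is off.
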(fn `InitGameState`
  (params (E_Maps :type "/Game/Blueprints/Enum/E_Maps Enum" :default "NewEnumerator0") (E_DIfficulties :type "/Game/Blueprints/Enum/E_Difficulties Enum" :default "NewEnumerator0"))
  (`|ExecutionSequence`
    (:`then_0`
      (switch `/Game/Blueprints/Enum/E_Maps` E_Maps
        (:`NewEnumerator0`
          (set `self.bIsOpenArea` false))
        (:`NewEnumerator1`
          (set `self.bIsOpenArea` true))))
    (:`then_1`
      (switch `/Game/Blueprints/Enum/E_Difficulties` E_DIfficulties
        (:`NewEnumerator0`
          (set `self.bIsVibration` false)
          (set `self.bIsNoise` false)
          (set `self.bIsDynamicWind` false))
        (:`NewEnumerator1`
          (set `self.bIsVibration` true)
          (set `self.bIsNoise` false)
          (set `self.bIsDynamicWind` false))
        (:`NewEnumerator2`
          (set `self.bIsVibration` false)
          (set `self.bIsNoise` true)
          (set `self.bIsDynamicWind` false))
        (:`NewEnumerator3`
          (set `self.bIsVibration` true)
          (set `self.bIsNoise` true)
          (set `self.bIsDynamicWind` false))
        (:`NewEnumerator4`
          (set `self.bIsVibration` true)
          (set `self.bIsNoise` true)
          (set `self.bIsDynamicWind` true))))
    (:`then_2`
      (`self.UpdateWind`))))

(fn `UpdateWind`
  (if (not (`self.bIsDynamicWind`))
    (set `self.WindDirection` (`KismetMathLibrary.RandomUnitVector`))))

(fn `UserConstructionScript`)